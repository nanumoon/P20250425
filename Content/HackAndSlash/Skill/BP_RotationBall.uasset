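; BP_RotationBall is a hack-and-slash skill actor: a ball that orbits its owning Character and damages what it passes near.
; Each tick it rotates its SpringArm to swing the Ball around and snaps the actor to the Character's location.
; An accumulated delay periodically applies radial damage at the Ball, ignoring the Character and crediting its controller.
; A timer started on BeginPlay destroys the actor after a few seconds.
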(event EventBeginPlay
  (Utilities|Time|SetTimerbyFunctionName 0 "DoDestroy" 5.0))

(event EventTick
  (params (DeltaSeconds :type Float%20%28single-precision%29))
  (Utilities|FlowControl|Sequence
    (:then_0
      (Transformation|AddRelativeRotation (Variables|Default|GetSpringArm) "0.000000,3.000000,0.000000" false false))
    (:then_1
      (Transformation|SetActorLocation (Transformation|GetActorLocation (Variables|Default|GetCharacter)) false false))
    (:then_2
      (CallFunction|UpdateDamage DeltaSeconds))))

(fn ConstructionScript
  (|CallParentFunction))

(fn UpdateDamage
  (params (DeltaSeconds :type Float%20%28double-precision%29))
  (bind _output_get (Variables|Default|SetDamageDelay (+ DeltaSeconds (Variables|Default|GetDamageDelay))))
  (if (> _output_get 0.1)
    (Variables|Default|SetDamageDelay 0.0)
    (Game|Damage|ApplyRadialDamage 1e+01 (Transformation|GetWorldLocation (Variables|Default|GetBall)) 1e+02 0 (Utilities|Array|MakeArray (Variables|Default|GetCharacter)) self (Pawn|GetController (Variables|Default|GetCharacter)) false "ECC_Visibility")))

(fn DoDestroy
  (Actor|DestroyActor))