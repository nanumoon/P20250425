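; Actor component that keeps spawning random monsters around its owner on the navmesh in the hack-and-slash game.
; A looping one-second timer started on BeginPlay calls DoSpawn, which picks a random DT_Monster row and a random navigable point within a very large radius.
; It spawns that row's MonsterClass with the BT_Mon behavior tree, then passes RandRowName to SetMonStat on BP_MonsterBase.
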(event EventBeginPlay
  (Utilities|Time|SetTimerbyFunctionName 0 "DoSpawn" 1.0 true))

(fn DoSpawn
  (bind _randomlocation (Class|NavigationSystemV1|GetRandomLocationinNavigableRadius (Transformation|GetActorLocation (Components|GetOwner)) 1e+05 0 0))
  (bind _outrownames (DataTable|GetDataTableRowNames "/Game/HackAndSlash/Monster/DT_Monster.DT_Monster"))
  (bind _returnvalue (Utilities|GetDataTableRow "/Game/HackAndSlash/Monster/DT_Monster.DT_Monster" (.OutItem (Utilities|Array|Random _outrownames)))
    (:then
      (bind _returnvalue_2 (AI|SpawnAIFromClass (.MonsterClass (Utilities|Struct|BreakST_Monster _returnvalue)) "/Game/HackAndSlash/AI/BT_Mon.BT_Mon" _randomlocation "0, 0, 0" false 0))
      (bind _asbp_monster_base (Utilities|Casting|CastToBP_MonsterBase _returnvalue_2))
      (Default|SetMonStat _asbp_monster_base (LocalVariables|GetRandRowName)))))